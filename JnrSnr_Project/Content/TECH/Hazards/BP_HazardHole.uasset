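; BP_HazardHole is a hole hazard that grows wider when other holes share its location.
; On BeginPlay it triggers CannonFX on the first BP_EnemyShip found in the level, if one exists.
; Every Tick, UpdateSize searches all actors of its class, counts others at nearly the same location, and widens the Hole component in X and Y per overlapping hole, keeping Z fixed.
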(event EventBeginPlay
  (|CallParentFunction)
  (bind _outactors (Actor|GetAllActorsOfClass "/Game/TECH/Hazards/BP_EnemyShip.BP_EnemyShip_C"))
  (if (>= (Utilities|Array|Length _outactors) 1)
    (Default|CannonFX (Utilities|Array|Get(acopy) _outactors))))

(event EventTick
  (params (DeltaSeconds :type Float%20%28single-precision%29))
  (CallFunction|UpdateSize))

(fn ConstructionScript
  (|CallParentFunction))

(fn UpdateSize
  (LocalVariables|SetnearbyHoleCount 0)
  (bind _outactors (Actor|GetAllActorsOfClass (Utilities|GetClass self)))
  (for _array_element _outactors
    (if (and (!= _array_element self) (Math|Vector|Equal(Vector) (Transformation|GetActorLocation _array_element) (Transformation|GetActorLocation) 0.5))
      (Math|Integer|IncrementInt (LocalVariables|GetnearbyHoleCount))))
  (Transformation|SetRelativeScale3D (Variables|Default|Gethole) (Math|Vector|MakeVector (.x (* "1.000000,1.000000,1.000000" (+ 1.0 (* (LocalVariables|GetnearbyHoleCount) 0.5)))) (.y (* "1.000000,1.000000,1.000000" (+ 1.0 (* (LocalVariables|GetnearbyHoleCount) 0.5)))) 1.0)))