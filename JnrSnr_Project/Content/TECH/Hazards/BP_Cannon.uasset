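; BP_Cannon is a cannon hazard that, when resolved, fires a shot at the enemy ship.
; Resolve plays the cannon sound, sets ShotFired and briefly shows the BANG component through TempBang and RemoveBang.
; After the flash it finds all BP_EnemyShip actors and calls Shot on the ship only if exactly one exists.
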(event EventResolve
  (Audio|PlaySound2D "/Game/DESIGN/Audio/cannon1.cannon1" 1.0 1.0 0.0 0 0)
  (Variables|Default|SetshotFired true)
  (CallFunction|TempBang)
  (Utilities|FlowControl|Delay 0.5)
  (CallFunction|RemoveBang)
  (bind _outactors (Actor|GetAllActorsOfClass "/Game/TECH/Hazards/BP_EnemyShip.BP_EnemyShip_C"))
  (if (== (Utilities|Array|Length _outactors) 1)
    (Default|Shot (Utilities|Array|Get(acopy) _outactors))))

(fn ConstructionScript
  (|CallParentFunction))

(fn TempBang
  (if (not (and (Rendering|IsVisible (Variables|Default|GetBANG)) (Math|Boolean|NotEqual(Boolean) (Variables|Default|GetshotFired) true)))
    (Rendering|SetVisibility (Variables|Default|GetBANG) true false)))

(fn RemoveBang
  (Rendering|SetVisibility (Variables|Default|GetBANG) false false))