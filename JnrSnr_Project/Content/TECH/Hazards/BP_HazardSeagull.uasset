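; Seagull hazard that flies across the play area, leaves a splat and slows players who touch it.
; Initialize plays a sound and starts a timeline that lerps the gull along a fixed path, revealing the splat past halfway and hiding the gull at the end.
; Splat zone overlap, not gated on the reveal, shows the BP_Movement splat decal and reduces movement speeds, restoring hardcoded values after a delay.
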(event OnComponentBeginOverlap(splat_zone)
  (params (OverlappedComponent :type Primitive%20Component%20Object%20Reference) (OtherActor :type Actor%20Object%20Reference) (OtherComp :type Primitive%20Component%20Object%20Reference) (OtherBodyIndex :type Integer) (bFromSweep :type Boolean) (SweepResult :type Hit%20Result%20Structure%20%28by%20ref%29))
  (bind _asbp_movement (Utilities|Casting|CastToBP_Movement OtherActor))
  (Rendering|SetVisibility (Variables|/Game/TECH/Pirates/BP_Movement.BP_Movement_C|GetplayerSplatdecal _asbp_movement) true false)
  (Variables|/Game/TECH/Pirates/BP_Movement.BP_Movement_C|SetUpDownSpeed _asbp_movement "0,0.300000, 0")
  (Variables|/Game/TECH/Pirates/BP_Movement.BP_Movement_C|SetLeftRightSpeed _asbp_movement "-0.300000, 0, 0")
  (Utilities|FlowControl|Delay 3.0)
  (Rendering|SetVisibility (Variables|/Game/TECH/Pirates/BP_Movement.BP_Movement_C|GetplayerSplatdecal _asbp_movement) false false)
  (Variables|/Game/TECH/Pirates/BP_Movement.BP_Movement_C|SetUpDownSpeed _asbp_movement "0,1.000000, 0")
  (Variables|/Game/TECH/Pirates/BP_Movement.BP_Movement_C|SetLeftRightSpeed _asbp_movement "-1.000000, 0, 0"))

(event EventInitialize
  (|CallParentFunction)
  (Audio|PlaySound2D "/Game/DESIGN/Audio/Seagull2.Seagull2" 1.0 1.0 0.0 0 0)
  (bind _alpha (Timeline|Timeline_0 PlayFromStart)
    (:Update
      (Transformation|SetRelativeLocation (Variables|Default|GetGull) (Math|Vector|Lerp(Vector) "800.000000,-1400.000000,300.000000" "-800.000000,1400.000000,300.000000" _alpha) false false)
      (if (and (> _alpha 0.5) (not (Variables|Default|GetinPlay)))
        (Variables|Default|SetinPlay true)
        (Rendering|SetVisibility (Variables|Default|Getsplat_2) true true)))
    (:Finished
      (Rendering|SetVisibility (Variables|Default|GetGull) false false))))

(fn ConstructionScript
  (|CallParentFunction))