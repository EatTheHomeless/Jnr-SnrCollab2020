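; Island hazard that drifts into place, positioned according to the HazardLevel of the first Tiller actor found.
; Green picks a random possible location, Red the death location, and Orange chooses between them at even odds, while Yellow behaves like Green.
; It registers with GameModeAAC, then a timeline slides the mesh in from an offset.
; Damage stays zero during the drift; death placements then restore the cached damage, others resolve.
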(event Custom|Drift
  (bind _alpha (Timeline|Timeline_0 PlayFromStart)
    (:Update
      (Transformation|SetRelativeLocation (Variables|Default|GetStaticMeshComponent10) (Math|Vector|Lerp(Vector) "-12000.000000,0.000000, 0" "0.000000,0.000000, 0" _alpha) false false))
    (:Finished
      (if (Variables|Default|GetdestinedToKill)
        (Variables|Default|SethazardDamage (Variables|Default|GetdestinedDamage))
        (else
          (CallFunction|Resolve))))))

(event EventInitialize
  (bind _possiblelocations (Variables|Default|GetpossibleLocations))
  (bind _outactors (Actor|GetAllActorsOfClass "/Game/DESIGN/Steering/Tiller.Tiller_C"))
  (if (>= (Utilities|Array|Length _outactors) 1)
    (switch Utilities|FlowControl|Switch|SwitchonHazardLevel (Variables|/Game/DESIGN/Steering/Tiller.Tiller_C|GetHazard%20level (Utilities|Array|Get(acopy) _outactors))
      (:NewEnumerator0
        (Transformation|SetActorLocation (Utilities|Array|Get(acopy) _possiblelocations (Math|Random|RandomInteger (Utilities|Array|Length _possiblelocations))) false false :!label _label)
        (Variables|Default|SetdestinedToKill false))
      (:NewEnumerator1
        (goto _label))
      (:NewEnumerator2
        (if (>= 0.5 (Math|Random|RandomFloat))
          (goto _label)
          (else
            (Transformation|SetActorLocation (Variables|Default|GetdeathLocation) false false :!label _label_2)
            (Variables|Default|SetdestinedToKill true))))
      (:NewEnumerator3
        (goto _label_2)))
    (Variables|Default|SethazardDamage 0.0)
    (bind _asgame_mode_aac (Utilities|Casting|CastToGameModeAAC (Game|GetGameMode)))
    (Default|AddActiveHazard _asgame_mode_aac self)
    (CallFunction|Drift)))

(event EventResolve
  (|CallParentFunction))

(fn ConstructionScript
  (|CallParentFunction)
  (Variables|Default|SetdestinedDamage (Variables|Default|GethazardDamage)))