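; BP_HazardFire is a fire hazard that periodically damages overlapping BP_Movement actors and grows visually when fires stack.
; Each Tick calls UpdateDamage, whose Delay throttles damage to DamagePerSecond scaled by UpdateSpeed.
; Tick also runs UpdateSize, which counts same-class actors at virtually the same location and enlarges the particle system by half its original scale per extra fire.
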(event Custom|UpdateDamage
  (Utilities|FlowControl|Delay (Variables|Default|GetupdateSpeed))
  (for _array_element (Collision|GetOverlappingActors 0 :!class /Script/Engine.Actor)
    (bind _asbp_movement (Utilities|Casting|CastToBP_Movement _array_element))
    (Game|Damage|ApplyDamage _asbp_movement (* (Variables|Default|GetdamagePerSecond) (Variables|Default|GetupdateSpeed)) 0 0)))

(event Collision|EventActorBeginOverlap
  (params (OtherActor :type Actor%20Object%20Reference))
  (|CallParentFunction OtherActor))

(event EventTick
  (params (DeltaSeconds :type Float%20%28single-precision%29))
  (CallFunction|UpdateSize)
  (CallFunction|UpdateDamage)
  (|CallParentFunction 0.0))

(fn ConstructionScript
  (|CallParentFunction)
  (Variables|Default|SetoriginalParticleScale (Variables|/Script/Engine.SceneComponent|GetRelativeScale3D (Variables|Default|GetParticleSystem))))

(fn UpdateSize
  (LocalVariables|SetnearbyFireCount 0)
  (bind _outactors (Actor|GetAllActorsOfClass (Utilities|GetClass self)))
  (for _array_element _outactors
    (if (and (!= _array_element self) (Math|Vector|Equal(Vector) (Transformation|GetActorLocation _array_element) (Transformation|GetActorLocation) 0.0001))
      (Math|Integer|IncrementInt (LocalVariables|GetnearbyFireCount))))
  (Transformation|SetRelativeScale3D (Variables|Default|GetParticleSystem) (* (Variables|Default|GetoriginalParticleScale) (+ 1.0 (* (LocalVariables|GetnearbyFireCount) 0.5)))))