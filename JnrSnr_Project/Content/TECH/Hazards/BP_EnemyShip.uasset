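; Enemy ship hazard that slides into position, takes hits and sinks away when defeated.
; Initialize runs an entry timeline that moves the mesh, then sets InPlay unless already resolving.
; Shot decrements ShotsLeft and calls Resolve at zero, which plays a descending, tilting timeline before handing off to the parent's resolve.
; CannonFX fires a particle burst at one of eleven random cannon points with a 2D sound.
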(event EventInitialize
  (|CallParentFunction)
  (bind _alpha (Timeline|Timeline_0 PlayFromStart)
    (:Update
      (Transformation|SetRelativeLocation (Variables|Default|GetStaticMesh) (Math|Vector|Lerp(Vector) "6500.000000,1200.000000, 0" "1000.000000,1200.000000, 0" _alpha) false false))
    (:Finished
      (if (not (Variables|Default|Getresolving))
        (Variables|Default|SetinPlay true)))))

(event EventResolve
  (bind _staticmesh (Variables|Default|GetStaticMesh))
  (Variables|Default|Setresolving true)
  (Variables|Default|SetinPlay false)
  (bind _alpha (Timeline|Timeline_1 PlayFromStart)
    (:Update
      (Transformation|SetRelativeLocation _staticmesh (Math|Vector|Lerp(Vector) "1000.000000,0.000000, 0" "4000.000000,0.000000,-3000.000000" _alpha) false false)
      (Transformation|SetRelativeRotation _staticmesh (Math|Rotator|Lerp(Rotator) "0,90.000000,0.000000" "0.000000,90.000000,-40.000000" _alpha) false false))
    (:Finished
      (|CallParentFunction))))

(fn ConstructionScript
  (|CallParentFunction))

(fn Shot
  (bind _shotsleft (Variables|Default|GetshotsLeft))
  (Math|Integer|DecrementInt _shotsleft
    (:%20%20
      (if (<= _shotsleft 0)
        (CallFunction|Resolve))
      (return))))

(fn CannonFX
  (switch int (Math|Random|RandomInteger 11)
    (:0
      (LocalVariables|SetChosenCannon (Variables|Default|GetCannonPoint)))
    (:1
      (LocalVariables|SetChosenCannon (Variables|Default|GetCannonPoint1)))
    (:2
      (LocalVariables|SetChosenCannon (Variables|Default|GetCannonPoint2)))
    (:3
      (LocalVariables|SetChosenCannon (Variables|Default|GetCannonPoint3)))
    (:4
      (LocalVariables|SetChosenCannon (Variables|Default|GetCannonPoint4)))
    (:5
      (LocalVariables|SetChosenCannon (Variables|Default|GetCannonPoint5)))
    (:6
      (LocalVariables|SetChosenCannon (Variables|Default|GetCannonPoint6)))
    (:7
      (LocalVariables|SetChosenCannon (Variables|Default|GetCannonPoint7)))
    (:8
      (LocalVariables|SetChosenCannon (Variables|Default|GetCannonPoint8)))
    (:9
      (LocalVariables|SetChosenCannon (Variables|Default|GetCannonPoint9)))
    (:10
      (LocalVariables|SetChosenCannon (Variables|Default|GetCannonPoint10))))
  (Effects|SpawnEmitteratLocation "/Game/ART/Particles/CannonVFX/Cannon.Cannon" (Transformation|GetWorldLocation (LocalVariables|GetChosenCannon)) "0.000000,180.000000, 0")
  (Audio|PlaySound2D "/Game/DESIGN/Audio/cannon1.cannon1" 1.0 1.0 0.0 0 0))