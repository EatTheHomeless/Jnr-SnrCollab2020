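; BP_HazardBase is a base hazard actor that registers with GameModeAAC and spawns at one of several predefined locations.
; Its construction script prints an on-screen warning when the PossibleLocations array is empty.
; Initialize adds the hazard to the game mode's active hazards and teleports it to a random entry from that array.
; Resolve removes it from the active hazards and destroys the actor.
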(fn ConstructionScript
  (if (== (Utilities|Array|Length (Variables|Default|GetpossibleLocations)) 0)
    (Development|PrintString (Utilities|String|Append (Utilities|GetDisplayName self) " has no possible spawn locations! Set them in the class defaults.") true true "(R=1.000000,G=0.000000,B=0.000000,A=1.000000)" 1e+01)))

(fn Initialize
  (bind _possiblelocations (Variables|Default|GetpossibleLocations))
  (bind _asgame_mode_aac (Utilities|Casting|CastToGameModeAAC (Game|GetGameMode))
    (:then
      (Default|AddActiveHazard _asgame_mode_aac self)
      (Transformation|SetActorLocation (Utilities|Array|Get(acopy) _possiblelocations (Math|Random|RandomInteger (Utilities|Array|Length _possiblelocations))) false false))
    (:CastFailed
      _))
  (return))

(fn Resolve
  (bind _asgame_mode_aac (Utilities|Casting|CastToGameModeAAC (Game|GetGameMode))
    (:then
      (Default|RemoveActiveHazard _asgame_mode_aac self))
    (:CastFailed
      _))
  (Actor|DestroyActor)
  (return))