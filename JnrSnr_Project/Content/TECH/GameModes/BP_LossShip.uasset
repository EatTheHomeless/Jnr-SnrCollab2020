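; BP_LossShip is an actor that stages a ship-sinking shot, presumably shown when the player loses.
; SinkShip switches player 0's view to this actor and plays a timeline from the start.
; The timeline's alpha interpolates the ship mesh's relative position and rotation so it moves downward and tilts, while rotating the camera alongside it.
; All start and end transforms are hard-coded.
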(event Custom|SinkShip
  (bind _staticmesh (Variables|Default|GetStaticMesh))
  (Game|Player|SetViewTargetwithBlend (Game|GetPlayerController 0) self 0.0 "VTBlend_Linear" 0.0 false)
  (bind _alpha (Timeline|Timeline_0 PlayFromStart)
    (:Update
      (Transformation|SetRelativeLocation _staticmesh (Math|Vector|Lerp(Vector) "1000.000000,1200.000000, 0" "4000.000000,1200.000000,-3000.000000" _alpha) false false)
      (Transformation|SetRelativeRotation _staticmesh (Math|Rotator|Lerp(Rotator) "0,90.000000,0.000000" "0.000000,90.000000,-40.000000" _alpha) false false)
      (Transformation|SetRelativeRotation (Variables|Default|GetCamera) (Math|Rotator|Lerp(Rotator) "-35.000000,60.000000,0.000000" "-35.000000,35.000000,0.000000" _alpha) false false))))

(fn ConstructionScript)