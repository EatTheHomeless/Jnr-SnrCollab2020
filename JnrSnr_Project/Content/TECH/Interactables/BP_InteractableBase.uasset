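; Base interactable item that a BP_Movement actor can pick up, carry and use to resolve hazards.
; Overlaps register it as the carrier's NearItem when free, or track a NearHazard matching its HazardToSolve class when held.
; Use resolves that hazard, with flags to disable, return to its construction-time location or destroy it afterward.
; Dropping attempts Use first, then detaches unless a successful use is set to keep holding.
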(event Custom|Returned
  (Transformation|DetachFromActor "KeepWorld" "KeepWorld" "KeepWorld")
  (Transformation|SetActorLocation (Variables|Default|GetoriginalLoc) false false)
  (Variables|Default|Setheld false))

(event Custom|PickedUp
  (params (AttachLoc :type Scene%20Component%20Object%20Reference))
  (Transformation|AttachComponentToComponent AttachLoc "None" "SnapToTarget" "KeepWorld" "KeepWorld" true)
  (Variables|Default|Setheld true))

(event Collision|EventActorBeginOverlap
  (params (OtherActor :type Actor%20Object%20Reference))
  (if (Variables|Default|Getheld)
    (if (== (Variables|Default|GethazardToSolve) (Utilities|GetClass OtherActor))
      (bind _asbp_hazard_base (Utilities|Casting|CastToBP_HazardBase OtherActor))
      (Variables|Default|SetnearHazard _asbp_hazard_base))
    (else
      (bind _asbp_movement (Utilities|Casting|CastToBP_Movement OtherActor))
      (Utilities|IsValid (Variables|/Game/TECH/Pirates/BP_Movement.BP_Movement_C|GetheldItem _asbp_movement)
        (:Is%20Not%20Valid
          (Utilities|IsValid (Variables|/Game/TECH/Pirates/BP_Movement.BP_Movement_C|GetnearItem _asbp_movement)
            (:Is%20Not%20Valid
              (Variables|/Game/TECH/Pirates/BP_Movement.BP_Movement_C|SetnearItem _asbp_movement self))))))))

(event Collision|EventActorEndOverlap
  (params (OtherActor :type Actor%20Object%20Reference))
  (if (Variables|Default|Getheld)
    (if (== OtherActor (Variables|Default|GetnearHazard)) :!label _label
      (Variables|Default|SetnearHazard 0))
    (else
      (bind _asbp_movement (Utilities|Casting|CastToBP_Movement OtherActor)
        (:then
          (if (not (== (Variables|/Game/TECH/Pirates/BP_Movement.BP_Movement_C|GetheldItem _asbp_movement) self))
            (Variables|/Game/TECH/Pirates/BP_Movement.BP_Movement_C|SetnearItem _asbp_movement 0)))
        (:CastFailed
          (goto _label))))))

(fn ConstructionScript
  (Variables|Default|SetoriginalLoc (Transformation|GetActorLocation)))

(fn Use
  (params (User :type BP%20Movement%20Object%20Reference))
  (bind _nearhazard (Variables|Default|GetnearHazard))
  (if (Variables|Default|Getusable)
    (Utilities|IsValid _nearhazard
      (:Is%20Valid
        (Default|Resolve _nearhazard)
        (if (Variables|Default|GetunusableAfterUse)
          (Variables|Default|Setusable false))
        (if (Variables|Default|GetreturnAfterUse)
          (CallFunction|Returned)
          (Default|ForgetItem User)
          (elif (Variables|Default|GetdestroyAfterUse)
            (Actor|DestroyActor)))
        (return true))
      (:Is%20Not%20Valid
        _)))
  (return false))

(fn Dropped
  (params (user :type BP%20Movement%20Object%20Reference))
  (bind _used (CallFunction|Use user))
  (if (or (not _used) (not (Variables|Default|GetkeepHoldingAfterUse)))
    (Transformation|DetachFromActor "KeepWorld" "KeepWorld" "KeepWorld")
    (Variables|Default|Setheld false)
    (return true)
    (else
      (return false))))