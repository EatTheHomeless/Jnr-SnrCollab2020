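; BP_InteractableBucket is an interactable bucket that can be refilled and shows whether it holds water.
; Overlapping an actor whose class exactly matches RefillActor sets Usable to true, after the parent overlap logic runs.
; Tick mirrors Usable onto the visibility of the Water component every frame, after the parent tick.
; This graph never clears Usable and otherwise defers to its parent class.
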(event Collision|EventActorBeginOverlap
  (params (OtherActor :type Actor%20Object%20Reference))
  (|CallParentFunction OtherActor)
  (if (== (Utilities|GetClass OtherActor) (Variables|Default|GetrefillActor))
    (Variables|Default|Setusable true)))

(event EventTick
  (params (DeltaSeconds :type Float%20%28single-precision%29))
  (|CallParentFunction DeltaSeconds)
  (Rendering|SetVisibility (Variables|Default|GetWater) (Variables|Default|Getusable) false))

(fn ConstructionScript
  (|CallParentFunction))