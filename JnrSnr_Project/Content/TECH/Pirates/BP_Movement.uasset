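; Player-controlled pirate character that walks on fixed world axes, picks up and drops items, and can die.
; Tick turns the mesh toward input, feeds run and carry flags to the female pirate AnimBP, regenerates health and checks a kill height.
; Damage pauses regeneration via a retriggerable delay; death returns held items, notifies BP_PirateController and leaves the camera's watch list.
; It also hosts temporary pause-menu and ship-hull UI.
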(event Custom|Initialize
  (Variables|Default|Setinitialized true))

(event Custom|DropItem
  (bind _dropped (Default|Dropped (Variables|Default|GetheldItem) self))
  (if _dropped
    (Variables|Default|SetheldItem 0)
    (Audio|PlaySound2D "/Game/DESIGN/Audio/inspectorj__pop.inspectorj__pop" 1.0 1.0 0.0 0 0)
    (Variables|Default|SetPickedUp false)))

(event Custom|PickUpItem
  (bind _output_get (Variables|Default|SetheldItem (Variables|Default|GetnearItem)))
  (Utilities|IsValid _output_get
    (:Is%20Valid
      (Default|PickedUp _output_get (Variables|Default|GetHoldingLoc))
      (Audio|PlaySound2D "/Game/DESIGN/Audio/inspectorj__pop.inspectorj__pop" 1.0 1.0 0.0 0 0)
      (Variables|Default|SetPickedUp true))))

(event Custom|ForgetItem
  (Variables|Default|SetnearItem 0))

(event Custom|RegenHealth
  (Utilities|FlowControl|Delay 0.2)
  (if (not (Variables|Default|GettakingDamage))
    (Variables|Default|Sethealth (Math|Float|Clamp(Float) (+ (Variables|Default|Gethealth) (* (Variables|Default|GethealthRegen) (Variables|Default|GetupdateSpeed))) 0.0 (Variables|Default|GetmaxHealth)))))

(event EventTick
  (params (DeltaSeconds :type Float%20%28single-precision%29))
  (CallFunction|CarryWalkAnim)
  (CallFunction|PickUpAnim)
  (CallFunction|AnimationSetup)
  (CallFunction|RegenHealth)
  (CallFunction|CheckKillZ)
  (Utilities|IsValid self
    (:Is%20Valid
      (if (or (!= (Input|AxisValues|GetUpDown) 0.0) (!= (Input|AxisValues|GetLeftRight) 0.0))
        (Variables|Default|Setdirection (Math|Vector|MakeVector (Input|AxisValues|GetUpDown) (Input|AxisValues|GetLeftRight) 0.0))
        (Transformation|SetWorldRotation (Variables|Character|GetMesh) (Math|Rotator|Lerp(Rotator) (Transformation|GetWorldRotation (Variables|Character|GetMesh)) (Math|Conversions|RotationFromXVector (Variables|Default|Getdirection)) (* DeltaSeconds (Variables|Default|GetrotationSpeed)) true) false false)))))

(event Game|Damage|EventAnyDamage
  (params (Damage :type Float%20%28single-precision%29) (DamageType :type Damage%20Type%20Object%20Reference) (InstigatedBy :type Controller%20Object%20Reference) (DamageCauser :type Actor%20Object%20Reference))
  (Utilities|FlowControl|FlipFlop
    (:A
      (Audio|PlaySound2D "/Game/DESIGN/Audio/gruntsound.gruntsound" 1.0 1.0 0.0 0 0))
    (:B
      (Audio|PlaySound2D "/Game/DESIGN/Audio/_soft-grunt._soft-grunt" 1.0 1.0 0.0 0 0)))
  (bind _output_get (Variables|Default|Sethealth (- (Variables|Default|Gethealth) Damage)))
  (if (<= _output_get 0.0)
    (Audio|PlaySound2D "/Game/DESIGN/Audio/grunt1-death-pain.grunt1-death-pain" 1.0 1.0 0.0 0 0)
    (CallFunction|Death)
    (else
      (Variables|Default|SettakingDamage true)
      (Utilities|FlowControl|RetriggerableDelay (Variables|Default|GetregenHaltTime))
      (Variables|Default|SettakingDamage false))))

(event EventBeginPlay
  ;[1 1 1] Temp Ship Health UI
  (bind _returnvalue (UserInterface|CreateWidget "/Game/TECH/UI/HUDElements/HullUI.HullUI_C"))
  (bind _output_get (Variables|Default|SetHullUIRef _returnvalue))
  (UserInterface|Viewport|AddtoViewport _output_get 0))

(event Input|ActionEvents|InputActionInteract
  (params (Key :type Key%20Structure))
  (:Pressed
    (Utilities|IsValid (Variables|Default|GetheldItem)
      (:Is%20Valid
        (CallFunction|DropItem))
      (:Is%20Not%20Valid
        (CallFunction|PickUpItem)))))

(event Input|ActionEvents|InputActionPause
  (params (Key :type Key%20Structure))
  (bind _returnvalue (Game|GetPlayerController 0))
  ;[1 1 1] Temp Pause
  (:Pressed
    (Utilities|IsValid (Variables|Default|GetPauseMenuRef)
      (:Is%20Valid
        _)
      (:Is%20Not%20Valid
        (bind _returnvalue_2 (UserInterface|CreateWidget "/Game/TECH/UI/PauseMenu.PauseMenu_C"))
        (Variables|Default|SetPauseMenuRef _returnvalue_2)))
    (Variables|/Script/Engine.PlayerController|SetbShowMouseCursor _returnvalue true)
    (Input|SetInputModeUIOnly _returnvalue (Variables|Default|GetPauseMenuRef) "DoNotLock")
    (UserInterface|Viewport|AddtoViewport (Variables|Default|GetPauseMenuRef) 0)
    (Game|SetGamePaused true)))

(event Input|AxisEvents|InputAxisUpDown
  (params (AxisValue :type Float%20%28single-precision%29))
  (Pawn|Input|AddMovementInput "0.000000,1.000000,0.000000" AxisValue false))

(event Input|AxisEvents|InputAxisLeftRight
  (params (AxisValue :type Float%20%28single-precision%29))
  (Pawn|Input|AddMovementInput "-1.000000,0.000000, 0" AxisValue false))

(fn ConstructionScript
  (Variables|Default|Sethealth (Variables|Default|GetmaxHealth)))

(fn Death
  (bind _helditem (Variables|Default|GetheldItem))
  (Utilities|IsValid _helditem
    (:Is%20Valid
      (Default|Returned _helditem))
    (:Is%20Not%20Valid
      _))
  (bind _asbp_pirate_controller (Utilities|Casting|CastToBP_PirateController (Pawn|GetController))
    (:then
      (Default|Death _asbp_pirate_controller))
    (:CastFailed
      _))
  (Default|RemoveActortoWatch (Variables|Default|GetpirateCamera) self)
  (Actor|DestroyActor)
  (return))

(fn CheckKillZ
  (if (<= (.z (Transformation|GetActorLocation)) (Variables|Default|GetkillZ))
    (CallFunction|Death))
  (return))

(fn AnimationSetup
  (bind _mesh (Variables|Character|GetMesh))
  (bind _returnvalue (Components|SkeletalMesh|GetAnimInstance _mesh))
  (if (or (!= (Input|AxisValues|GetLeftRight) 0.0) (!= (Input|AxisValues|GetUpDown) 0.0))
    (bind _asabp_female_pirate (Utilities|Casting|CastToABP_Female_Pirate _returnvalue))
    (Variables|/Game/ANIMATION/Female/ABP_Female_Pirate.ABP_Female_Pirate_C|SetCanRun _asabp_female_pirate true)
    (else
      (bind _asabp_female_pirate_2 (Utilities|Casting|CastToABP_Female_Pirate _returnvalue))
      (Variables|/Game/ANIMATION/Female/ABP_Female_Pirate.ABP_Female_Pirate_C|SetCanRun _asabp_female_pirate_2 false))))

(fn PickUpAnim
  (bind _mesh (Variables|Character|GetMesh))
  (bind _returnvalue (Components|SkeletalMesh|GetAnimInstance _mesh))
  (if (Variables|Default|GetPickedUp)
    (bind _asabp_female_pirate (Utilities|Casting|CastToABP_Female_Pirate _returnvalue))
    (Variables|/Game/ANIMATION/Female/ABP_Female_Pirate.ABP_Female_Pirate_C|SetPickingUp _asabp_female_pirate true)
    (else
      (bind _asabp_female_pirate_2 (Utilities|Casting|CastToABP_Female_Pirate _returnvalue))
      (Variables|/Game/ANIMATION/Female/ABP_Female_Pirate.ABP_Female_Pirate_C|SetPickingUp _asabp_female_pirate_2 false))))

(fn CarryWalkAnim
  (bind _mesh (Variables|Character|GetMesh))
  (bind _returnvalue (Components|SkeletalMesh|GetAnimInstance _mesh))
  (if (and (or (!= (Input|AxisValues|GetLeftRight) 0.0) (!= (Input|AxisValues|GetUpDown) 0.0)) (Variables|Default|GetPickedUp))
    (bind _asabp_female_pirate (Utilities|Casting|CastToABP_Female_Pirate _returnvalue))
    (Variables|/Game/ANIMATION/Female/ABP_Female_Pirate.ABP_Female_Pirate_C|SetcarryWalkAnim _asabp_female_pirate true)
    (else
      (bind _asabp_female_pirate_2 (Utilities|Casting|CastToABP_Female_Pirate _returnvalue))
      (Variables|/Game/ANIMATION/Female/ABP_Female_Pirate.ABP_Female_Pirate_C|SetcarryWalkAnim _asabp_female_pirate_2 false))))

(fn GetPlayerController
  (bind _asplayer_controller (Utilities|Casting|CastToPlayerController (Pawn|GetController))
    (:then
      (return _asplayer_controller))
    (:CastFailed
      (return 0))))

(fn GetPlayerMesh
  (return (Variables|Character|GetMesh)))