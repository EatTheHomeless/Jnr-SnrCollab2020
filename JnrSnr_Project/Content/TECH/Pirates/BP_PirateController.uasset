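; Player controller for pirate players that links each pawn to the level's single BP_PirateCamera and handles respawning.
; On BeginPlay it finds that camera and makes it the view target.
; Possession retries until the camera is set, registers the pawn as a watched actor, then initializes its BP_Movement with player ID and camera.
; On death it unpossesses, asks GameModeAAC for permission, then spawns and possesses a default pawn at a random PlayerStart after a delay.
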(event Custom|Death
  (Pawn|UnPossess)
  (bind _asgame_mode_aac (Utilities|Casting|CastToGameModeAAC (Game|GetGameMode))
    (:then
      (bind (_authorized _respawntime) (Default|RequestRespawn _asgame_mode_aac))
      (if _authorized
        (Utilities|FlowControl|Delay _respawntime)
        (bind _outactors (Actor|GetAllActorsOfClass "/Script/Engine.PlayerStart"))
        (bind _returnvalue (Game|SpawnActorfromClass (Variables|/Script/Engine.GameModeBase|GetDefaultPawnClass (Game|GetGameMode)) (Math|Transform|MakeTransform (Transformation|GetActorLocation (Utilities|Array|Get(acopy) _outactors (Math|Random|RandomInteger (Utilities|Array|Length _outactors)))) "0, 0, 0" "1,1,1") "Undefined" 0 0))
        (Pawn|Possess _returnvalue)))
    (:CastFailed
      (Development|PrintString "The gamemode of this level is not GameModeAAC! Have you set the GameMode defaults correctly?" true true "(R=1.000000,G=0.000000,B=0.000000,A=1.000000)" 1e+01))))

(event Custom|SetCamera
  (Development|PrintString (Utilities|String|Append "Player " (Utilities|String|ToString(Integer) (Class|GameplayStatics|GetPlayerControllerID self)) " added.") true true "(R=0.000000,G=0.660000,B=1.000000,A=1.000000)" 1e+01)
  (bind _outactors (Actor|GetAllActorsOfClass "/Game/TECH/Pirates/BP_PirateCamera.BP_PirateCamera_C"))
  (switch int (Utilities|Array|Length _outactors)
    (:Default
      (Development|PrintString "There are too many PirateCamera actors in the scene!" true true "(R=1.000000,G=0.000000,B=0.000000,A=1.000000)" 1e+01))
    (:0
      (Development|PrintString "Could not find a PirateCamera actor!" true true "(R=1.000000,G=0.000000,B=0.000000,A=1.000000)" 1e+01))
    (:1
      (Variables|Default|SetPirateCamera (Utilities|Array|Get(acopy) _outactors))
      (Game|Player|SetViewTargetwithBlend (Utilities|Array|Get(acopy) _outactors) 0.0 "VTBlend_Linear" 0.0 false))))

(event EventBeginPlay
  (CallFunction|SetCamera))

(event EventPossess
  (params (PossessedPawn :type Pawn%20Object%20Reference))
  (bind _piratecamera (Variables|Default|GetPirateCamera))
  (if (!= _piratecamera 0) :!label _label
    (Default|AddActortoWatch _piratecamera PossessedPawn)
    (bind _asbp_movement (Utilities|Casting|CastToBP_Movement PossessedPawn)
      (:then
        (if (not (Variables|/Game/TECH/Pirates/BP_Movement.BP_Movement_C|Getinitialized _asbp_movement))
          (Variables|/Game/TECH/Pirates/BP_Movement.BP_Movement_C|SetID _asbp_movement (Class|GameplayStatics|GetPlayerControllerID self))
          (Variables|/Game/TECH/Pirates/BP_Movement.BP_Movement_C|SetpirateCamera _asbp_movement (Variables|Default|GetPirateCamera))
          (Default|Initialize _asbp_movement)))
      (:CastFailed
        (Development|PrintString "The Pawn which PirateController has possessed is not a BP_Movement! Have you set the GameMode defaults correctly?" true true "(R=1.000000,G=0.000000,B=0.000000,A=1.000000)" 1e+01)))
    (else
      (Utilities|FlowControl|RetriggerableDelay 0.2)
      (goto _label))))

(fn ConstructionScript)