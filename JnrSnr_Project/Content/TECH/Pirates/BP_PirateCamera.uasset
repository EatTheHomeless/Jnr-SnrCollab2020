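; BP_PirateCamera is a camera actor for the Pirates game that keeps itself centered over a changeable list of watched actors.
; Each tick it computes the XY bounding box of those actors, optionally including a fixed central position, and interpolates toward the midpoint while keeping its height.
; Functions add, remove and query watched actors.
; The camera's original relative offset is cached at construction but not used in these graphs.
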(event EventTick
  (params (DeltaSeconds :type Float%20%28single-precision%29))
  (bind _topleftpos (Variables|Default|GetTopLeftPos))
  (bind _bottomrightpos (Variables|Default|GetBottomRightPos))
  (CallFunction|UpdateEdgePositions)
  (Transformation|SetActorLocation (Math|Interpolation|VInterpTo (Transformation|GetActorLocation) (Math|Vector|MakeVector (/ (+ (.x _topleftpos) (.x _bottomrightpos)) 2.0) (/ (+ (.y _topleftpos) (.y _bottomrightpos)) 2.0) (.z (Transformation|GetActorLocation))) DeltaSeconds (Variables|Default|GetLerpSpeed)) false true))

(fn ConstructionScript
  (Variables|Default|SetOriginalOffset (.location (Transformation|GetRelativeTransform (Variables|Default|GetCamera)))))

(fn AddActortoWatch
  (params (Actor :type Actor%20Object%20Reference))
  (Utilities|Array|Add (Variables|Default|GetActorsToWatch) Actor)
  (return))

(fn RemoveActortoWatch
  (params (Actor :type Actor%20Object%20Reference))
  (bind _actorstowatch (Variables|Default|GetActorsToWatch))
  (Utilities|Array|RemoveItem _actorstowatch Actor)
  (Development|PrintString (Utilities|String|Append "Removed " (Utilities|GetDisplayName Actor) " from ActorsToWatch in PirateCamera. New length: " (Utilities|String|ToString(Integer) (Utilities|Array|Length _actorstowatch))) true true "(R=0.000000,G=0.660000,B=1.000000,A=1.000000)" 1e+01))

(fn IsWatching
  (params (Actor :type Actor%20Object%20Reference))
  (return (Utilities|Array|ContainsItem (Variables|Default|GetActorsToWatch) Actor)))

(fn UpdateEdgePositions
  (bind _centralpos (Variables|Default|GetCentralPos))
  (Variables|Default|SetTopLeftPos _centralpos)
  (Variables|Default|SetBottomRightPos _centralpos)
  (for (_array_element _array_index) (Variables|Default|GetActorsToWatch)
    (if (and (== _array_index 0) (not (Variables|Default|GetUseCentralPos)))
      (Variables|Default|SetTopLeftPos (Math|Conversions|ToVector2D(Vector) (Transformation|GetActorLocation _array_element)))
      (Variables|Default|SetBottomRightPos (Math|Conversions|ToVector2D(Vector) (Transformation|GetActorLocation _array_element)))
      (else
        (if (> (.x (Transformation|GetActorLocation _array_element)) (.x (Variables|Default|GetTopLeftPos)))
          (Variables|Default|SetTopLeftPos (Math|Vector2D|MakeVector2D (.x (Transformation|GetActorLocation _array_element)) (.y (Variables|Default|GetTopLeftPos)))))
        (if (> (.y (Transformation|GetActorLocation _array_element)) (.y (Variables|Default|GetTopLeftPos)))
          (Variables|Default|SetTopLeftPos (Math|Vector2D|MakeVector2D (.x (Variables|Default|GetTopLeftPos)) (.y (Transformation|GetActorLocation _array_element)))))
        (if (< (.x (Transformation|GetActorLocation _array_element)) (.x (Variables|Default|GetBottomRightPos)))
          (Variables|Default|SetBottomRightPos (Math|Vector2D|MakeVector2D (.x (Transformation|GetActorLocation _array_element)) (.y (Variables|Default|GetBottomRightPos)))))
        (if (< (.y (Transformation|GetActorLocation _array_element)) (.y (Variables|Default|GetBottomRightPos)))
          (Variables|Default|SetBottomRightPos (Math|Vector2D|MakeVector2D (.x (Variables|Default|GetBottomRightPos)) (.y (Transformation|GetActorLocation _array_element))))))))
  (return))