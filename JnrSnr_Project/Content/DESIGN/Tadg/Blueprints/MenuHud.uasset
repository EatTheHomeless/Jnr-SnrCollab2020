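; Menu HUD Blueprint that creates and switches between the main menu, high score, controls and level select widgets.
; BeginPlay shows the main menu and sets InGame, which is passed to each main menu instance.
; Screen events call DisplayUI, which hides the current widget rather than removing it and creates a new one.
; It also forwards AnyKey results to the current widget and stores the selected level for FindLevel.
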(event EventBeginPlay
  (bind _returnvalue (UserInterface|CreateWidget "/Game/DESIGN/Tadg/Widgets/MainMenuWidget.MainMenuWidget_C" (Game|GetPlayerController 0)))
  (bind _output_get (Variables|Default|SetCurrent _returnvalue))
  (Variables|/Game/DESIGN/Tadg/Widgets/MainMenuWidget.MainMenuWidget_C|SetIngame _returnvalue (Variables|Default|GetInGame))
  (UserInterface|Viewport|AddtoPlayerScreen _output_get)
  (Variables|Default|SetInGame true))

(event EventAnyKey
  (params (Success :type Boolean))
  (Class|Interface2|AnyKey(Message) (Variables|Default|GetCurrent) Success))

(event EventMainMenu
  (params (Success :type Boolean))
  (bind _widget (CallFunction|DisplayUI (Variables|Default|GetCurrent) "/Game/DESIGN/Tadg/Widgets/MainMenuWidget.MainMenuWidget_C"))
  (bind _asmain_menu_widget (Utilities|Casting|CastToMainMenuWidget _widget))
  (Variables|/Game/DESIGN/Tadg/Widgets/MainMenuWidget.MainMenuWidget_C|SetIngame _asmain_menu_widget (Variables|Default|GetInGame)))

(event EventHighScore
  (params (LevelPos :type Integer))
  (Variables|Default|SetSelectedLevel LevelPos)
  (CallFunction|DisplayUI (Variables|Default|GetCurrent) "/Game/DESIGN/Tadg/Widgets/HighScore.HighScore_C"))

(event EventControls
  (CallFunction|DisplayUI (Variables|Default|GetCurrent) "/Game/DESIGN/Tadg/Widgets/Controls.Controls_C"))

(event EventLevel
  (CallFunction|DisplayUI (Variables|Default|GetCurrent) "/Game/DESIGN/Tadg/Widgets/LevelSelect.LevelSelect_C"))

(fn ConstructionScript)

(fn DisplayUI
  (params (Current :type Widget%20Object%20Reference) (NewParam1 :type User%20Widget%20Class%20Reference))
  (Widget|SetVisibility Current "Hidden")
  (bind _returnvalue (UserInterface|CreateWidget NewParam1 (Game|GetPlayerController 0)))
  (bind _output_get (Variables|Default|SetCurrent _returnvalue))
  (UserInterface|Viewport|AddtoPlayerScreen _output_get)
  (Widget|SetVisibility _output_get "Visible")
  (return _output_get))

(fn FindLevel
  (return (Variables|Default|GetSelectedLevel)))